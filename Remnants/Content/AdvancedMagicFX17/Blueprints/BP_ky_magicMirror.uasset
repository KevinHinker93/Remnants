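; BP_ky_magicMirror is a magic mirror effect actor from the AdvancedMagicFX17 set, with an adjustable secondary color.
; Both the construction script and BeginPlay create a dynamic material instance on element 1 of the Fx component and set its colorB parameter from SubColor.
; It then calls the parent logic at BeginPlay, and its overlap and tick events are unused.
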(event `self.ReceiveBeginPlay`
  ;[1 1 1] sub color control
  (bind _returnvalue (`PrimitiveComponent.CreateDynamicMaterialInstance` (`self.fx`) 1 null))
  (`MaterialInstanceDynamic.SetVectorParameterValue` _returnvalue "colorB" (`self.subColor`))
  (`parent.ReceiveBeginPlay`))

(fn `UserConstructionScript`
  (`parent.UserConstructionScript`)
  ;[1 1 1] sub color control
  (bind _returnvalue (`PrimitiveComponent.CreateDynamicMaterialInstance` (`self.fx`) 1 null))
  (`MaterialInstanceDynamic.SetVectorParameterValue` _returnvalue "colorB" (`self.subColor`)))