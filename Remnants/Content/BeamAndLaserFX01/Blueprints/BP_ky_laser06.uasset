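; BP_ky_laser06 is a laser effect actor that exposes highlight and spiral colors for its Fx component.
; The construction script creates a dynamic material instance on element 0 and sets its hilightColor parameter from HilightColor.
; It also passes SpiralColor, converted to a vector, into the effect's spiral vector parameter.
; The event graph holds only disabled stubs, so the actor has no runtime logic.
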(fn `UserConstructionScript`
  ;[1 1 1] get effect's material instance
  (`parent.UserConstructionScript`)
  (bind _returnvalue (`PrimitiveComponent.CreateDynamicMaterialInstance` (`self.fx`) 0 null))
  ;[1 1 1] set hilight color
  (`MaterialInstanceDynamic.SetVectorParameterValue` _returnvalue "hilightColor" (`self.hilightColor`))
  ;[1 1 1] set spiral color
  (`ParticleSystemComponent.SetVectorParameter` (`self.fx`) "spiral" (`KismetMathLibrary.Conv_LinearColorToVector` (`self.spiralColor`))))