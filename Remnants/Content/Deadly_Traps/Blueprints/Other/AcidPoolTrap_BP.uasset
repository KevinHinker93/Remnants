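; Acid pool trap that damages an actor tagged Player while it stands inside the pool collider.
; Entry applies one hit of the raw damage multiplier and starts a looping timer, which exit clears.
; Each tick deals the larger of the FirstPersonCharacter's max health or max shield times that multiplier, with a sound.
; All damage uses the lava damage type.
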(event `self.ReceiveBeginPlay`)

(event `self.PoolCollider.OnComponentBeginOverlap`
  (params (OverlappedComponent :type "PrimitiveComponent Object Reference") (OtherActor :type "Actor Object Reference") (OtherComp :type "PrimitiveComponent Object Reference") (OtherBodyIndex :type Integer) (bFromSweep :type Boolean) (SweepResult :type "HitResult Structure (by ref)"))
  (if (`self.ActorHasTag` OtherActor "Player")
    (set `self.ActorToDamage` OtherActor)
    (if (not (`KismetSystemLibrary.K2_TimerExistsHandle` (`self.damageTimerHandle`)))
      (`self.Damage` (`self.ActorToDamage`) (`self.poolDamageMult`))
      (bind _returnvalue (`KismetSystemLibrary.K2_SetTimerDelegate` (delegate `OnDamage`) (`self.damagePerSec`) true))
      (set `self.damageTimerHandle` _returnvalue))))

(event `OnDamage`
  (bind _actortodamage (`self.ActorToDamage`))
  (bind _asfirst_person_character (cast `/Game/FirstPersonCPP/Blueprints/Characters/Player/FirstPersonCharacter` (`self.ActorToDamage`)))
  (`self.Damage` _actortodamage (* (`KismetMathLibrary.Max` (`HealthComponent.m_maxHealth` (`ShootergameCharacter.m_healthComponent` _asfirst_person_character)) (`ShieldComponent.m_maxShield` (`ShootergameCharacter.m_shieldComponent` _asfirst_person_character))) (`self.poolDamageMult`)))
  (`GameplayStatics.PlaySoundAtLocation` "/Game/Sound/poolDamaged.poolDamaged" (`self.K2_GetActorLocation` _actortodamage)))

(event `self.PoolCollider.OnComponentEndOverlap`
  (params (OverlappedComponent :type "PrimitiveComponent Object Reference") (OtherActor :type "Actor Object Reference") (OtherComp :type "PrimitiveComponent Object Reference") (OtherBodyIndex :type Integer))
  (if (`self.ActorHasTag` OtherActor "Player")
    (set `self.ActorToDamage` null)
    (`KismetSystemLibrary.K2_ClearAndInvalidateTimerHandle` (`self.damageTimerHandle`))))

(fn `Damage`
  (params (actorToDamage :type "Actor Object Reference") (damage :type "Float (double-precision)"))
  (`GameplayStatics.ApplyDamage` actorToDamage damage null null "/Game/FirstPersonCPP/Blueprints/DamageTypes/Lava/LavaDamageTypeA_BP.LavaDamageTypeA_BP_C"))

(fn `UserConstructionScript`)