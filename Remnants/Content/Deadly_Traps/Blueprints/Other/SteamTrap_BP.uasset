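; Steam trap actor that cycles on and off using interval and duration delays, toggling its collider, beam particle, decoration and sound.
; A player-tagged actor entering while active takes default steam damage immediately, then a looping timer applies repeated hits.
; Repeat hits on FirstPersonCharacter scale with the larger of max health or max shield.
; The timer clears on end overlap; the deactivate function does not clear it.
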(event `TrapDeactivate`
  (`self.DeactivateSteamTrap`)
  (`KismetSystemLibrary.Delay` (`self.trapInterval`))
  (`self.TrapActivate`))

(event `TrapActivate`
  (`self.ActivateSteamTrap`)
  (`KismetSystemLibrary.Delay` (`self.trapDuration`))
  (`self.TrapDeactivate`))

(event `self.ReceiveBeginPlay`
  (`self.DeactivateSteamTrap`)
  (`KismetSystemLibrary.Delay` (`self.trapInterval`))
  (`self.TrapActivate`))

(event `self.PoolCollider.OnComponentBeginOverlap`
  (params (OverlappedComponent :type "PrimitiveComponent Object Reference") (OtherActor :type "Actor Object Reference") (OtherComp :type "PrimitiveComponent Object Reference") (OtherBodyIndex :type Integer) (bFromSweep :type Boolean) (SweepResult :type "HitResult Structure (by ref)"))
  (if (`self.IsActive`)
    (if (`self.ActorHasTag` OtherActor "Player")
      (set `self.ActorToDamage` OtherActor)
      (if (not (`KismetSystemLibrary.K2_TimerExistsHandle` (`self.damageTimerHandle`)))
        (`self.Damage` (`self.ActorToDamage`) (`self.poolDefaultDamage`))
        (bind _returnvalue (`KismetSystemLibrary.K2_SetTimerDelegate` (delegate `OnDamage`) (`self.damagePerSec`) true))
        (set `self.damageTimerHandle` _returnvalue)))))

(event `OnDamage`
  (bind _actortodamage (`self.ActorToDamage`))
  (`/Engine/EditorBlueprintResources/StandardMacros.IsValid` _actortodamage
    (:`Is Valid`
      (bind _asfirst_person_character (cast `/Game/FirstPersonCPP/Blueprints/Characters/Player/FirstPersonCharacter` _actortodamage)
        (:`then`
          (`self.Damage` _actortodamage (* (`KismetMathLibrary.Max` (`HealthComponent.m_maxHealth` (`ShootergameCharacter.m_healthComponent` _asfirst_person_character)) (`ShieldComponent.m_maxShield` (`ShootergameCharacter.m_shieldComponent` _asfirst_person_character))) (`self.damageMult`))))
        (:`CastFailed`
          (`self.Damage` _actortodamage (`self.poolDefaultDamage`)))))))

(event `self.PoolCollider.OnComponentEndOverlap`
  (params (OverlappedComponent :type "PrimitiveComponent Object Reference") (OtherActor :type "Actor Object Reference") (OtherComp :type "PrimitiveComponent Object Reference") (OtherBodyIndex :type Integer))
  (if (`self.ActorHasTag` OtherActor "Player")
    (set `self.ActorToDamage` null)
    (`KismetSystemLibrary.K2_ClearAndInvalidateTimerHandle` (`self.damageTimerHandle`))))

(fn `ActivateSteamTrap`
  (`ActorComponent.Activate` (`self.PoolCollider`) true)
  (`ActorComponent.Activate` (`self.BeamParticle`) true)
  (`ActorComponent.Activate` (`self.Deco`) true)
  (`ActorComponent.Activate` (`self.SteamSound`) true)
  (set `self.IsActive` true))

(fn `Damage`
  (params (actorToDamage :type "Actor Object Reference") (damage :type "Float (double-precision)"))
  (`GameplayStatics.ApplyDamage` actorToDamage damage null null "/Game/FirstPersonCPP/Blueprints/DamageTypes/Steam/SteamDamageTypeA_BP.SteamDamageTypeA_BP_C"))

(fn `DeactivateSteamTrap`
  (`ActorComponent.Deactivate` (`self.Deco`))
  (`ActorComponent.Deactivate` (`self.BeamParticle`))
  (`ActorComponent.Deactivate` (`self.PoolCollider`))
  (`ActorComponent.Deactivate` (`self.SteamSound`))
  (set `self.IsActive` false))

(fn `UserConstructionScript`)